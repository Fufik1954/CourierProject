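; BP_Marker is a waypoint marker that shows an icon and the player's distance to it through a WB_Waypoint widget.
; On BeginPlay it applies the marker's icon texture and color to the widget and starts a looping timer.
; The timer periodically writes the distance to the player pawn as whole meters with a Russian "м" suffix, avoiding Tick.
; StopDistanceUpdates clears that timer.
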(event `self.ReceiveBeginPlay`
  ; Получаем текстовое поле
  (bind _aswb_waypoint (cast `/Game/UI/WB_Waypoint` (`WidgetComponent.GetWidget` (`self.Widget`))))
  (set `self.Distancetext` (`/Game/UI/WB_Waypoint.Distancetext` _aswb_waypoint))
  (bind _iconimage (`/Game/UI/WB_Waypoint.IconImage` _aswb_waypoint))
  (`Image.SetBrush` _iconimage (`WidgetBlueprintLibrary.MakeBrushFromTexture` (`self.MarkerIcon`)))
  (`Image.SetColorAndOpacity` _iconimage (`self.MarkerColor`))
  (bind _returnvalue (`KismetSystemLibrary.K2_SetTimerDelegate` (delegate `UpdateDistance`) 0.2 true))
  (set `self.TimerHandle` _returnvalue))

(event `UpdateDistance`
  ; Записываем дистанцию в текстовое поле
  (`TextBlock.SetText` (`self.Distancetext`) (`KismetTextLibrary.Conv_StringToText` (`KismetStringLibrary.Concat_StrStr` (`KismetStringLibrary.Conv_IntToString` (`KismetMathLibrary.FTrunc` (/ (`KismetMathLibrary.Vector_Distance` (`self.K2_GetActorLocation`) (`self.K2_GetActorLocation` (`GameplayStatics.GetPlayerPawn` 0))) 100.0))) " м"))))

(event `StopDistanceUpdates`
  (if (`KismetSystemLibrary.K2_IsValidTimerHandle` (`self.TimerHandle`))
    (`KismetSystemLibrary.K2_ClearAndInvalidateTimerHandle` (`self.TimerHandle`))))

(fn `UserConstructionScript`)