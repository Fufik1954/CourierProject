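; BP_PickupSpot is a delivery pickup point that spawns a package and map-style marker at BeginPlay.
; A trigger overlap toggles the interaction zone flag and the player's HUD prompt.
; Interact attaches the package to the player's hand socket, picks a random house and starts the delivery timer, refusing if already carrying or none is available.
; After pickup, a delayed respawn spawns a replacement package.
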(event `self.ReceiveBeginPlay`
  ; Спавн посылки на старте
  (bind _returnvalue (`|SpawnActorFromClass` "/Game/Blueprints/BP_Package.BP_Package_C" (`KismetMathLibrary.MakeTransform` (+ (`self.K2_GetActorLocation`) (`self.SpawnVector`)) (struct :`Yaw` 180.0)) "Undefined" "MultiplyWithRoot" null null))
  (set `self.SpawnedPackage` _returnvalue)
  (set `self.bIsPackageAvailable` true)
  (`|SpawnActorFromClass` "/Game/Blueprints/BP_Marker.BP_Marker_C" (`KismetMathLibrary.Conv_VectorToTransform` (+ (`self.K2_GetActorLocation`) (0.0 0.0 100.0))) "Undefined" "MultiplyWithRoot" null "/Game/UI/Sprite/Point2.Point2" (struct :`R` 1.0 :`G` 0.012983 :`A` 1.0) null))

(event `/Game/Interface/BI_Interactable.Interact`
  (params (Instigator :type "/Game/ThirdPerson/Blueprints/BP_ThirdPersonCharacter Object Reference"))
  (bind _spawnedpackage (`self.SpawnedPackage`))
  (bind _spawnedpackage_2 (`self.SpawnedPackage`))
  (bind _localplayer (`self.LocalPlayer`))
  ; Логика взятия посылки
  (if (`self.bPlayerInInteractionZone`)
    (bind _output_get (set `self.LocalPlayer` Instigator))
    (if (not (`/Game/ThirdPerson/Blueprints/BP_ThirdPersonCharacter.bHasPackage` _output_get))
      (if (`self.bIsPackageAvailable`)
        (`self.K2_AttachToComponent` _spawnedpackage (`Character.Mesh` (`self.LocalPlayer`)) "PackageSocket" "SnapToTarget" "KeepRelative" "KeepRelative" true)
        (`self.K2_SetActorRelativeRotation` _spawnedpackage (struct :`Yaw` -90.0 :`Roll` 90.0) false false)
        (set `/Game/ThirdPerson/Blueprints/BP_ThirdPersonCharacter.bHasPackage` true _localplayer)
        (`/Game/ThirdPerson/Blueprints/BP_ThirdPersonCharacter.SelectRandomHouse` _localplayer)
        (`/Game/ThirdPerson/Blueprints/BP_ThirdPersonCharacter.UpdateOrderStatus ` _localplayer)
        (set `self.bIsPackageAvailable` false)
        (set `/Game/ThirdPerson/Blueprints/BP_ThirdPersonCharacter.CurrentPackage ` _spawnedpackage_2 _localplayer)
        (`/Game/ThirdPerson/Blueprints/BP_ThirdPersonCharacter.StartDeliveryTimer` _localplayer)
        (`PrimitiveComponent.SetCollisionProfileName` (`/Game/Blueprints/BP_Package.Cube` _spawnedpackage_2) "NoCollision" true)
        (set `self.SpawnedPackage` null)
        (`self.RespawnPackage`)
        (set `self.LocalPlayer` null)
        (`GameplayStatics.PlaySound2D` (`self.TakeOrderSound`) 1.0 1.0 0.0 null null)
        (else
          (`KismetSystemLibrary.PrintString` "Новых посылок еще нет")
          (`GameplayStatics.PlaySound2D` (`self.AlreadyHasPackage`) 1.0 1.0 0.0 null null :!label _label)))
      (else
        (`KismetSystemLibrary.PrintString` "Посылка уже есть")
        (goto _label)))
    (else
      (`KismetSystemLibrary.PrintString` "Войди в нужную зону"))))

(event `RespawnPackage`
  ; Респавн после взятия
  (`KismetSystemLibrary.Delay` (`self.RespawnTimer`))
  (`/Engine/EditorBlueprintResources/StandardMacros.IsValid` (`self.SpawnedPackage`)
    (:`Is Not Valid`
      (bind _returnvalue (`|SpawnActorFromClass` "/Game/Blueprints/BP_Package.BP_Package_C" (`KismetMathLibrary.MakeTransform` (+ (`self.K2_GetActorLocation`) (`self.SpawnVector`)) (struct :`Yaw` 180.0)) "Undefined" "MultiplyWithRoot" null null))
      (set `self.SpawnedPackage` _returnvalue)
      (set `self.bIsPackageAvailable` true)
      (`KismetSystemLibrary.PrintString` "Доступна новая посылка"))))

(event `self.PickupTrigger.OnComponentBeginOverlap`
  (params (OverlappedComponent :type "PrimitiveComponent Object Reference") (OtherActor :type "Actor Object Reference") (OtherComp :type "PrimitiveComponent Object Reference") (OtherBodyIndex :type Integer) (bFromSweep :type Boolean) (SweepResult :type "HitResult Structure (by ref)"))
  ; Обработка коллизии
  (bind _asbp_third_person_character (cast `/Game/ThirdPerson/Blueprints/BP_ThirdPersonCharacter` OtherActor))
  (set `self.bPlayerInInteractionZone` true)
  (`/Game/UI/Game/WBP_MainHUD.ShowInteractPrompt` (`/Game/ThirdPerson/Blueprints/BP_ThirdPersonCharacter.HUD` _asbp_third_person_character) (`self.Text`)))

(event `self.PickupTrigger.OnComponentEndOverlap`
  (params (OverlappedComponent :type "PrimitiveComponent Object Reference") (OtherActor :type "Actor Object Reference") (OtherComp :type "PrimitiveComponent Object Reference") (OtherBodyIndex :type Integer))
  ; Обработка коллизии
  (bind _asbp_third_person_character (cast `/Game/ThirdPerson/Blueprints/BP_ThirdPersonCharacter` OtherActor))
  (set `self.bPlayerInInteractionZone` false)
  (`/Game/UI/Game/WBP_MainHUD.HideInteractPrompt` (`/Game/ThirdPerson/Blueprints/BP_ThirdPersonCharacter.HUD` _asbp_third_person_character)))

(fn `UserConstructionScript`)