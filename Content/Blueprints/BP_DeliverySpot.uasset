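; BP_DeliverySpot is a house drop-off point where the player completes timed package deliveries for coins.
; Interact checks the player's target house ID, carried package and remaining time, then detaches the package and places it at the drop location.
; Success pays a base reward plus capped time bonus, resets the player's delivery state and destroys the package after a delay.
; It also spawns and removes its own BP_Marker waypoint.
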(event `Interact`
  (params (`InstigatorPlayer ` :type "/Game/ThirdPerson/Blueprints/BP_ThirdPersonCharacter Object Reference"))
  ; Вызов
  (set `self.LocalPlayer` `InstigatorPlayer `)
  (`self.ValidateDelivery`))

(event `ValidateDelivery`
  ; Проверка условий и установление значений
  (if (== (`/Game/ThirdPerson/Blueprints/BP_ThirdPersonCharacter.TargetHouseID` (`self.LocalPlayer`)) (`self.HouseID`))
    (if (`/Game/ThirdPerson/Blueprints/BP_ThirdPersonCharacter.bHasPackage` (`self.LocalPlayer`))
      (if (> (`/Game/ThirdPerson/Blueprints/BP_ThirdPersonCharacter.CurrentTime` (`self.LocalPlayer`)) 0.0)
        (bind _output_get (set `self.DroppedPackage` (`/Game/ThirdPerson/Blueprints/BP_ThirdPersonCharacter.CurrentPackage ` (`self.LocalPlayer`))))
        (`self.K2_DetachFromActor` _output_get "KeepRelative" "KeepRelative" "KeepRelative")
        (`self.K2_SetActorLocation` (`self.DroppedPackage`) (`SceneComponent.K2_GetComponentLocation` (`self.PackageDropLocation `)) false false)
        (`PrimitiveComponent.SetCollisionProfileName` (`/Game/Blueprints/BP_Package.Cube` (`self.DroppedPackage`)) "BlockAllDynamic" true)
        (`self.ProcessSuccess`)))
    (else
      (`KismetSystemLibrary.PrintString` "Дом неправильный"))))

(event `ProcessSuccess`
  (bind _returnvalue (`KismetMathLibrary.Min` (`KismetMathLibrary.FTrunc` (`/Game/ThirdPerson/Blueprints/BP_ThirdPersonCharacter.CurrentTime` (`self.LocalPlayer`))) 50))
  ; Награда
  (`/Game/ThirdPerson/Blueprints/BP_ThirdPersonCharacter.AddCoins ` (`self.LocalPlayer`) (+ _returnvalue 100))
  (`KismetSystemLibrary.PrintString` (`KismetStringLibrary.Concat_StrStr` "Заказ доставлен! +100 моент," "+ бонус: " (`KismetStringLibrary.Conv_IntToString` _returnvalue)))
  (`self.ResetDeliveryState`)
  (`GameplayStatics.PlaySound2D` (`self.DeliverySuccessSound`) 1.0 1.0 0.0 null null))

(event `ResetDeliveryState`
  (bind _localplayer (`self.LocalPlayer`))
  ; Очищение/обнуление/удаление
  (set `/Game/ThirdPerson/Blueprints/BP_ThirdPersonCharacter.CurrentPackage ` null _localplayer)
  (set `/Game/ThirdPerson/Blueprints/BP_ThirdPersonCharacter.bHasPackage` false _localplayer)
  (set `/Game/ThirdPerson/Blueprints/BP_ThirdPersonCharacter.TargetHouseID` 0 _localplayer)
  (`/Game/ThirdPerson/Blueprints/BP_ThirdPersonCharacter.StopDeliveryTimer` _localplayer)
  (`self.DeleteMarker`)
  (set `self.LocalPlayer` null)
  (`KismetSystemLibrary.PrintString` "Переменные очищены")
  (`KismetSystemLibrary.Delay` (`self.DeleteTimer`))
  (`self.K2_DestroyActor` (`self.DroppedPackage`))
  (set `self.DroppedPackage` null))

(event `SpawnMarker`
  ; Установка маркера
  (bind _returnvalue (`|SpawnActorFromClass` "/Game/Blueprints/BP_Marker.BP_Marker_C" (`KismetMathLibrary.Conv_VectorToTransform` (+ (`self.K2_GetActorLocation`) (`self.VectorSpawn`))) "Undefined" "MultiplyWithRoot" null null))
  (set `self.WaypointMarkerClass` _returnvalue))

(event `DeleteMarker`
  (`self.K2_DestroyActor` (`self.WaypointMarkerClass`))
  (set `self.WaypointMarkerClass` null))

(fn `UserConstructionScript`)