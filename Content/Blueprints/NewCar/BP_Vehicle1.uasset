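; Drivable Chaos wheeled vehicle that the player can enter, drive and exit, carrying a package in its trunk.
; Overlap triggers show prompts and gate Interact, which either boards the car, moving any held package to the trunk, or retrieves it at the trunk.
; Entering hides and attaches the character, swaps input mapping contexts and possesses the car; exiting reverses this at ExitPoint.
; A spawned marker hides while driving, and engine audio pitch follows RPM.
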(event `HandlePackageOnEnter`
  (bind `_сurrentplayer` (`self.СurrentPlayer`))
  (bind _packageintrunk (`self.PackageInTrunk`))
  (bind _currentpackage_ (`/Game/ThirdPerson/Blueprints/BP_ThirdPersonCharacter.CurrentPackage ` (`self.СurrentPlayer`)))
  ; Кладем посылку в багажник
  (`/Engine/EditorBlueprintResources/StandardMacros.IsValid` _currentpackage_
    (:`Is Valid`
      (bind _output_get (set `self.PackageInTrunk` _currentpackage_))
      (`self.K2_DetachFromActor` _output_get "KeepRelative" "KeepRelative" "KeepRelative")
      (`self.K2_AttachToComponent` (`self.PackageInTrunk`) (`self.TrunkAttachPoint`) "TrunkAttachPoint" "KeepRelative" "KeepRelative" "KeepRelative" true)
      (`self.K2_SetActorRelativeRotation` :`self` _packageintrunk)
      (`SceneComponent.SetRelativeScale3D` (`/Game/Blueprints/BP_Package.Cube` _packageintrunk) (1.0 0.4 1.0))
      (set `self.bHasPackageInTrunk` true)
      (set `/Game/ThirdPerson/Blueprints/BP_ThirdPersonCharacter.CurrentPackage ` null `_сurrentplayer`)
      (set `/Game/ThirdPerson/Blueprints/BP_ThirdPersonCharacter.bHasPackage` false `_сurrentplayer`))))

(event `EnhancedInput|/Game/Input/Actions/Car/IA_LookUp`
  (params (ActionValue :type "Float (double-precision)") (ElapsedSeconds :type "Float (double-precision)") (TriggeredSeconds :type "Float (double-precision)") (InputAction :type "InputAction Object Reference" :default "/Game/Input/Actions/Car/IA_LookUp.IA_LookUp"))
  ; Камера
  (:`Triggered`
    (`self.AddControllerPitchInput` ActionValue)))

(event `EnhancedInput|/Game/Input/Actions/Car/IA_LookRight`
  (params (ActionValue :type "Float (double-precision)") (ElapsedSeconds :type "Float (double-precision)") (TriggeredSeconds :type "Float (double-precision)") (InputAction :type "InputAction Object Reference" :default "/Game/Input/Actions/Car/IA_LookRight.IA_LookRight"))
  ; Камера
  (:`Triggered`
    (`self.AddControllerYawInput` ActionValue)))

(event `TakePackageFromTrunk`
  (bind _packageintrunk (`self.PackageInTrunk`))
  (bind _packageintrunk_2 (`self.PackageInTrunk`))
  ; Забираем посылку с багажника
  (if (`self.bHasPackageInTrunk`)
    (`/Engine/EditorBlueprintResources/StandardMacros.IsValid` _packageintrunk
      (:`Is Valid`
        (`self.K2_DetachFromActor` _packageintrunk "KeepRelative" "KeepRelative" "KeepRelative")
        (`self.K2_AttachToComponent` (`self.PackageInTrunk`) (`Character.Mesh` (`self.СurrentPlayer`)) "PackageSocket" "SnapToTarget" "KeepRelative" "KeepRelative" true)
        (`self.K2_SetActorRelativeRotation` _packageintrunk_2 (struct :`Yaw` -90.0 :`Roll` 90.0) false false)
        (`SceneComponent.SetRelativeScale3D` (`/Game/Blueprints/BP_Package.Cube` _packageintrunk_2) (0.7 0.7 0.7))
        (set `/Game/ThirdPerson/Blueprints/BP_ThirdPersonCharacter.CurrentPackage ` (`self.PackageInTrunk`) (`self.СurrentPlayer`))
        (set `/Game/ThirdPerson/Blueprints/BP_ThirdPersonCharacter.bHasPackage` true (`self.СurrentPlayer`))
        (set `self.PackageInTrunk` null)
        (set `self.bHasPackageInTrunk` false)))))

(event `EnhancedInput|/Game/Input/Actions/Car/IA_HandBrake`
  (params (ActionValue :type "Float (double-precision)") (ElapsedSeconds :type "Float (double-precision)") (TriggeredSeconds :type "Float (double-precision)") (InputAction :type "InputAction Object Reference" :default "/Game/Input/Actions/Car/IA_HandBrake.IA_HandBrake"))
  (bind _vehiclemovementcomponent (`self.VehicleMovementComponent`))
  ; Ручник
  (:`Started`
    (`ChaosVehicleMovementComponent.SetHandbrakeInput` _vehiclemovementcomponent true)
    (set `self.bHandbrakeActive` true)
    (`ChaosVehicleMovementComponent.SetThrottleInput` _vehiclemovementcomponent 0.0)
    (`ChaosVehicleMovementComponent.SetBrakeInput` _vehiclemovementcomponent 1.0))
  (:`Completed`
    (`ChaosVehicleMovementComponent.SetHandbrakeInput` _vehiclemovementcomponent false)
    (set `self.bHandbrakeActive` false)
    (`ChaosVehicleMovementComponent.SetBrakeInput` _vehiclemovementcomponent 0.0)))

(event `self.Interact`
  (params (Instigator :type "/Game/ThirdPerson/Blueprints/BP_ThirdPersonCharacter Object Reference"))
  ; Вызов
  (if (`self.bPlayerInInteractionZone`)
    (if (not (`self.bIsOccupied`))
      (bind _output_get (set `self.СurrentPlayer` Instigator))
      (set `/Game/ThirdPerson/Blueprints/BP_ThirdPersonCharacter.CurrentVehicle ` self _output_get)
      (`self.EnterVehicle` _output_get)
      (`self.HandlePackageOnEnter`)
      (`self.SetActorHiddenInGame` (`self.Marker`) true)
      (bind _output_get_2 (set `self.TextVehicle` "[F] чтобы выйти из машины"))
      (`/Game/UI/Game/WBP_MainHUD.ShowInteractPrompt` (`/Game/ThirdPerson/Blueprints/BP_ThirdPersonCharacter.HUD` (`self.СurrentPlayer`)) _output_get_2)
      (`AudioComponent.Play` (`self.Engine`) 0.0))
    (elif (`self.bPlayerInInteractionZoneTrunk`)
      (`self.TakePackageFromTrunk `))))

(event `EnhancedInput|/Game/Input/Actions/Car/IA_MoveForward`
  (params (ActionValue :type "Float (double-precision)") (ElapsedSeconds :type "Float (double-precision)") (TriggeredSeconds :type "Float (double-precision)") (InputAction :type "InputAction Object Reference" :default "/Game/Input/Actions/Car/IA_MoveForward.IA_MoveForward"))
  (bind _vehiclemovementcomponent (`self.VehicleMovementComponent`))
  ; Газ/Тормоз
  (:`Triggered`
    (if (>= ActionValue 0.0)
      (`ChaosVehicleMovementComponent.SetThrottleInput` _vehiclemovementcomponent ActionValue)
      (`ChaosVehicleMovementComponent.SetBrakeInput` _vehiclemovementcomponent 0.0)
      (elif (not (`self.bHandbrakeActive`))
        (`ChaosVehicleMovementComponent.SetBrakeInput` _vehiclemovementcomponent (* ActionValue -1.0))
        (`ChaosVehicleMovementComponent.SetThrottleInput` _vehiclemovementcomponent 0.0)))))

(event `self.EnterTrigger.OnComponentBeginOverlap`
  (params (OverlappedComponent :type "PrimitiveComponent Object Reference") (OtherActor :type "Actor Object Reference") (OtherComp :type "PrimitiveComponent Object Reference") (OtherBodyIndex :type Integer) (bFromSweep :type Boolean) (SweepResult :type "HitResult Structure (by ref)"))
  ; Обработка коллизии для посадки/высадки машины
  (bind _asbp_third_person_character (cast `/Game/ThirdPerson/Blueprints/BP_ThirdPersonCharacter` OtherActor))
  (set `self.bPlayerInInteractionZone` true)
  (`/Game/UI/Game/WBP_MainHUD.ShowInteractPrompt` (`/Game/ThirdPerson/Blueprints/BP_ThirdPersonCharacter.HUD` _asbp_third_person_character) (`self.TextVehicle`)))

(event `self.TrunkTrigger.OnComponentBeginOverlap`
  (params (OverlappedComponent :type "PrimitiveComponent Object Reference") (OtherActor :type "Actor Object Reference") (OtherComp :type "PrimitiveComponent Object Reference") (OtherBodyIndex :type Integer) (bFromSweep :type Boolean) (SweepResult :type "HitResult Structure (by ref)"))
  ; Обработка коллизии багажника
  (bind _asbp_third_person_character (cast `/Game/ThirdPerson/Blueprints/BP_ThirdPersonCharacter` OtherActor))
  (set `self.bPlayerInInteractionZoneTrunk` true)
  (bind _output_get (set `self.СurrentPlayer` _asbp_third_person_character))
  (`/Game/UI/Game/WBP_MainHUD.ShowInteractPrompt` (`/Game/ThirdPerson/Blueprints/BP_ThirdPersonCharacter.HUD` _output_get) (`self.TextTrunk`)))

(event `self.TrunkTrigger.OnComponentEndOverlap`
  (params (OverlappedComponent :type "PrimitiveComponent Object Reference") (OtherActor :type "Actor Object Reference") (OtherComp :type "PrimitiveComponent Object Reference") (OtherBodyIndex :type Integer))
  ; Обработка коллизии багажника
  (cast `/Game/ThirdPerson/Blueprints/BP_ThirdPersonCharacter` OtherActor)
  (set `self.bPlayerInInteractionZoneTrunk` false)
  (`/Game/UI/Game/WBP_MainHUD.HideInteractPrompt` (`/Game/ThirdPerson/Blueprints/BP_ThirdPersonCharacter.HUD` (`self.СurrentPlayer`)))
  (set `self.СurrentPlayer` null))

(event `self.EnterTrigger.OnComponentEndOverlap`
  (params (OverlappedComponent :type "PrimitiveComponent Object Reference") (OtherActor :type "Actor Object Reference") (OtherComp :type "PrimitiveComponent Object Reference") (OtherBodyIndex :type Integer))
  ; Обработка коллизии для посадки/высадки машины
  (bind _asbp_third_person_character (cast `/Game/ThirdPerson/Blueprints/BP_ThirdPersonCharacter` OtherActor))
  (set `self.bPlayerInInteractionZone` false)
  (`/Game/UI/Game/WBP_MainHUD.HideInteractPrompt` (`/Game/ThirdPerson/Blueprints/BP_ThirdPersonCharacter.HUD` _asbp_third_person_character)))

(event `EnhancedInput|/Game/Input/Actions/Car/IA_MoveRight`
  (params (ActionValue :type "Float (double-precision)") (ElapsedSeconds :type "Float (double-precision)") (TriggeredSeconds :type "Float (double-precision)") (InputAction :type "InputAction Object Reference" :default "/Game/Input/Actions/Car/IA_MoveRight.IA_MoveRight"))
  (bind _vehiclemovementcomponent (`self.VehicleMovementComponent`))
  ; Лево/Право
  (:`Started`
    (`ChaosVehicleMovementComponent.SetSteeringInput` _vehiclemovementcomponent ActionValue))
  (:`Completed`
    (`ChaosVehicleMovementComponent.SetSteeringInput` _vehiclemovementcomponent 0.0)))

(event `EnhancedInput|/Game/Input/Actions/Car/IA_ExitVehicle`
  (params (ActionValue :type Boolean) (ElapsedSeconds :type "Float (double-precision)") (TriggeredSeconds :type "Float (double-precision)") (InputAction :type "InputAction Object Reference" :default "/Game/Input/Actions/Car/IA_ExitVehicle.IA_ExitVehicle"))
  (bind `_сurrentplayer` (`self.СurrentPlayer`))
  ; Выход из машины
  (:`Started`
    (if (`self.bIsOccupied`)
      (`/Game/UI/Game/WBP_MainHUD.HideInteractPrompt` (`/Game/ThirdPerson/Blueprints/BP_ThirdPersonCharacter.HUD` `_сurrentplayer`))
      (`self.ExitVehicle ` (`/Game/ThirdPerson/Blueprints/BP_ThirdPersonCharacter.OriginalPlayerController` `_сurrentplayer`))
      (`self.SetActorHiddenInGame` (`self.Marker`) false)
      (`AudioComponent.Stop` (`self.Engine`))
      (set `self.TextVehicle` "[E] чтобы сесть в машину"))))

(event `self.ReceiveBeginPlay`
  ; Создание маркера машины
  (bind _returnvalue (`|SpawnActorFromClass` "/Game/Blueprints/BP_Marker.BP_Marker_C" (`KismetMathLibrary.Conv_VectorToTransform` (`self.K2_GetActorLocation`)) "Undefined" "MultiplyWithRoot" null "/Game/UI/Sprite/Point3.Point3" (struct :`R` 0.5 :`G` 0.119399 :`B` 0.011487 :`A` 1.0) null))
  (bind _output_get (set `self.Marker` _returnvalue))
  (`self.K2_AttachToActor` _output_get self "Marker" "SnapToTarget" "SnapToTarget" "SnapToTarget" true)
  (`AudioComponent.Stop` (`self.Engine`)))

(event `self.ReceiveTick`
  (params (DeltaSeconds :type "Float (single-precision)"))
  (bind _aschaos_wheeled_vehicle_movement_component (cast `ChaosWheeledVehicleMovementComponent` (`self.VehicleMovementComponent`)))
  (`AudioComponent.SetPitchMultiplier` (`self.Engine`) (`KismetMathLibrary.MapRangeClamped` (`ChaosWheeledVehicleMovementComponent.GetEngineRotationSpeed` _aschaos_wheeled_vehicle_movement_component) 800.0 6000.0 0.6 2.0)))

(fn `EnterVehicle`
  (params (Player :type "/Game/ThirdPerson/Blueprints/BP_ThirdPersonCharacter Object Reference"))
  (bind _returnvalue (`self.GetController` Player))
  (bind _asplayer_controller (cast `PlayerController` _returnvalue))
  (`|ExecutionSequence`
    (:`then_0`
      (`self.SetActorHiddenInGame` Player true)
      (`self.SetActorEnableCollision` Player false))
    (:`then_1`
      (bind _returnvalue_2 (pcsubsystem `EnhancedInputLocalPlayerSubsystem` _asplayer_controller))
      (`EnhancedInputSubsystemInterface.RemoveMappingContext` _returnvalue_2 "/Game/Input/IMC_Default.IMC_Default" (struct)))
    (:`then_2`
      (`EnhancedInputSubsystemInterface.AddMappingContext` _returnvalue_2 "/Game/Input/Actions/Car/IMC_Pickup.IMC_Pickup" 0 (struct)))
    (:`then_3`
      (set `self.bIsOccupied` true))
    (:`then_4`
      (`self.K2_AttachToActor` Player self "Player" "SnapToTarget" "SnapToTarget" "SnapToTarget" true)
      (`Controller.Possess` _returnvalue self))))

(fn `ExitVehicle `
  (params (PlayerController :type "PlayerController Object Reference"))
  (bind _returnvalue (pcsubsystem `EnhancedInputLocalPlayerSubsystem` PlayerController))
  (bind `_сurrentplayer` (`self.СurrentPlayer`))
  (bind `_сurrentplayer_2` (`self.СurrentPlayer`))
  (`|ExecutionSequence`
    (:`then_0`
      (`self.K2_DetachFromActor` `_сurrentplayer_2` "KeepRelative" "KeepRelative" "KeepRelative")
      (`self.K2_SetActorLocation` `_сurrentplayer_2` (+ (`SceneComponent.K2_GetComponentLocation` (`self.ExitPoint `)) (0.0 0.0 25.0)) false false)
      (`Controller.Possess` PlayerController `_сurrentplayer_2`))
    (:`then_1`
      (`self.SetActorHiddenInGame` `_сurrentplayer` false)
      (`self.SetActorEnableCollision` `_сurrentplayer` true))
    (:`then_2`
      (set `self.bIsOccupied` false)
      (set `self.СurrentPlayer` null))
    (:`then_3`
      (`EnhancedInputSubsystemInterface.RemoveMappingContext` _returnvalue "/Game/Input/Actions/Car/IMC_Pickup.IMC_Pickup" (struct)))
    (:`then_4`
      (`EnhancedInputSubsystemInterface.AddMappingContext` _returnvalue "/Game/Input/IMC_Default.IMC_Default" 0 (struct)))))

(fn `UserConstructionScript`)