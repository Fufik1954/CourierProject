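; Drivable pickup vehicle Blueprint that a player character can enter and exit.
; Enhanced Input actions drive camera look, throttle, brake, steering and handbrake; an active handbrake blocks negative forward input.
; EnterVehicle hides the character, disables its collision, attaches it to the Player socket, possesses the pickup and swaps mapping contexts.
; ExitVehicle detaches it at ExitPoint, restores possession, visibility, collision and default input.
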(event `EnhancedInput|/Game/Input/Actions/Car/IA_LookUp`
  (params (ActionValue :type "Float (double-precision)") (ElapsedSeconds :type "Float (double-precision)") (TriggeredSeconds :type "Float (double-precision)") (InputAction :type "InputAction Object Reference" :default "/Game/Input/Actions/Car/IA_LookUp.IA_LookUp"))
  ; Камера
  (:`Triggered`
    (`self.AddControllerPitchInput` ActionValue)))

(event `EnhancedInput|/Game/Input/Actions/Car/IA_LookRight`
  (params (ActionValue :type "Float (double-precision)") (ElapsedSeconds :type "Float (double-precision)") (TriggeredSeconds :type "Float (double-precision)") (InputAction :type "InputAction Object Reference" :default "/Game/Input/Actions/Car/IA_LookRight.IA_LookRight"))
  ; Камера
  (:`Triggered`
    (`self.AddControllerYawInput` ActionValue)))

(event `EnhancedInput|/Game/Input/Actions/Car/IA_HandBrake`
  (params (ActionValue :type "Float (double-precision)") (ElapsedSeconds :type "Float (double-precision)") (TriggeredSeconds :type "Float (double-precision)") (InputAction :type "InputAction Object Reference" :default "/Game/Input/Actions/Car/IA_HandBrake.IA_HandBrake"))
  (bind _vehiclemovementcomponent (`self.VehicleMovementComponent`))
  ; Ручник
  (:`Started`
    (`ChaosVehicleMovementComponent.SetHandbrakeInput` _vehiclemovementcomponent true)
    (set `self.bHandbrakeActive` true)
    (`ChaosVehicleMovementComponent.SetThrottleInput` _vehiclemovementcomponent 0.0)
    (`ChaosVehicleMovementComponent.SetBrakeInput` _vehiclemovementcomponent 1.0))
  (:`Completed`
    (`ChaosVehicleMovementComponent.SetHandbrakeInput` _vehiclemovementcomponent false)
    (set `self.bHandbrakeActive` false)
    (`ChaosVehicleMovementComponent.SetBrakeInput` _vehiclemovementcomponent 0.0)))

(event `EnhancedInput|/Game/Input/Actions/Car/IA_MoveForward`
  (params (ActionValue :type "Float (double-precision)") (ElapsedSeconds :type "Float (double-precision)") (TriggeredSeconds :type "Float (double-precision)") (InputAction :type "InputAction Object Reference" :default "/Game/Input/Actions/Car/IA_MoveForward.IA_MoveForward"))
  (bind _vehiclemovementcomponent (`self.VehicleMovementComponent`))
  ; Газ/Тормоз
  (:`Triggered`
    (if (>= ActionValue 0.0)
      (`ChaosVehicleMovementComponent.SetThrottleInput` _vehiclemovementcomponent ActionValue)
      (`ChaosVehicleMovementComponent.SetBrakeInput` _vehiclemovementcomponent 0.0)
      (elif (not (`self.bHandbrakeActive`))
        (`ChaosVehicleMovementComponent.SetBrakeInput` _vehiclemovementcomponent (* ActionValue -1.0))
        (`ChaosVehicleMovementComponent.SetThrottleInput` _vehiclemovementcomponent 0.0)))))

(event `EnhancedInput|/Game/Input/Actions/Car/IA_MoveRight`
  (params (ActionValue :type "Float (double-precision)") (ElapsedSeconds :type "Float (double-precision)") (TriggeredSeconds :type "Float (double-precision)") (InputAction :type "InputAction Object Reference" :default "/Game/Input/Actions/Car/IA_MoveRight.IA_MoveRight"))
  (bind _vehiclemovementcomponent (`self.VehicleMovementComponent`))
  ; Лево/Право
  (:`Started`
    (`ChaosVehicleMovementComponent.SetSteeringInput` _vehiclemovementcomponent ActionValue))
  (:`Completed`
    (`ChaosVehicleMovementComponent.SetSteeringInput` _vehiclemovementcomponent 0.0)))

(event `EnhancedInput|/Game/Input/Actions/Car/IA_ExitVehicle`
  (params (ActionValue :type Boolean) (ElapsedSeconds :type "Float (double-precision)") (TriggeredSeconds :type "Float (double-precision)") (InputAction :type "InputAction Object Reference" :default "/Game/Input/Actions/Car/IA_ExitVehicle.IA_ExitVehicle"))
  (:`Triggered`
    (if (`self.bIsOccupied`)
      (`self.ExitVehicle ` (`self.PlayerController`)))))

(fn `EnterVehicle`
  (params (Player :type "/Game/ThirdPerson/Blueprints/BP_ThirdPersonCharacter Object Reference") (PickUp :type "/Game/Blueprints/Car/BP_Pickup Object Reference"))
  (bind _currentplayer (`self.CurrentPlayer`))
  (if (not (`self.bIsOccupied`))
    (bind _output_get (set `self.CurrentPlayer` Player))
    (set `self.bIsOccupied` true)
    (bind _returnvalue (`self.GetController` _output_get))
    (bind _asplayer_controller (cast `PlayerController` _returnvalue))
    (`|ExecutionSequence`
      (:`then_0`
        (`self.SetActorHiddenInGame` _currentplayer true))
      (:`then_1`
        (`self.SetActorEnableCollision` _currentplayer false))
      (:`then_2`
        (bind _returnvalue_2 (pcsubsystem `EnhancedInputLocalPlayerSubsystem` _asplayer_controller))
        (`EnhancedInputSubsystemInterface.RemoveMappingContext` _returnvalue_2 "/Game/Input/IMC_Default.IMC_Default" (struct)))
      (:`then_3`
        (`EnhancedInputSubsystemInterface.AddMappingContext` _returnvalue_2 "/Game/Input/Actions/Car/IMC_Pickup.IMC_Pickup" 0 (struct)))
      (:`then_4`
        (`self.K2_AttachToActor` (`self.CurrentPlayer`) PickUp "Player" "SnapToTarget" "SnapToTarget" "SnapToTarget" true)
        (`Controller.Possess` _returnvalue PickUp)))))

(fn `ExitVehicle `
  (params (PlayerController :type "PlayerController Object Reference"))
  (bind _returnvalue (pcsubsystem `EnhancedInputLocalPlayerSubsystem` PlayerController))
  (bind _currentplayer (`self.CurrentPlayer`))
  (bind _currentplayer_2 (`self.CurrentPlayer`))
  (`|ExecutionSequence`
    (:`then_0`
      (`self.K2_DetachFromActor` _currentplayer_2 "KeepRelative" "KeepRelative" "KeepRelative")
      (`self.K2_SetActorLocation` _currentplayer_2 (`SceneComponent.K2_GetComponentLocation` (`self.ExitPoint `)) false false)
      (`Controller.Possess` PlayerController _currentplayer_2)
      (`KismetSystemLibrary.PrintString` "Деаттач"))
    (:`then_1`
      (`self.SetActorHiddenInGame` _currentplayer false))
    (:`then_2`
      (`self.SetActorEnableCollision` _currentplayer true))
    (:`then_3`
      (set `self.bIsOccupied` false)
      (set `self.CurrentPlayer` null))
    (:`then_4`
      (`EnhancedInputSubsystemInterface.RemoveMappingContext` _returnvalue "/Game/Input/Actions/Car/IMC_Pickup.IMC_Pickup" (struct)))
    (:`then_5`
      (`EnhancedInputSubsystemInterface.AddMappingContext` _returnvalue "/Game/Input/IMC_Default.IMC_Default" 0 (struct)))))

(fn `UserConstructionScript`)